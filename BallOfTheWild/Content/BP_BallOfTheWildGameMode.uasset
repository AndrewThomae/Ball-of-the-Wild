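; BP_BallOfTheWildGameMode is the game mode that tracks joined players and handles level change and respawn requests.
; PostLogin adds each BP_PlayerController to a unique PlayerControllers list.
; NewLevel calls NewWorld, which is defined outside these graphs.
; Respawn destroys the controller's pawn and spawns the given class at the world origin, owned by that controller, without possessing it here.
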(event Custom|NewLevel
  (Class|BallOftheWildGameMode|NewWorld))

(event Custom|Respawn
  (params (PlayerController :type Player%20Controller%20Object%20Reference) (Class :type BP%20Third%20Person%20Character%20Class%20Reference))
  (Actor|DestroyActor (Pawn|GetControlledPawn PlayerController))
  (Game|SpawnActorfromClass Class (Math|Transform|MakeTransform "0, 0, 0") "Undefined" PlayerController 0))

(event EventBeginPlay)

(event EventTick
  (params (DeltaSeconds :type Float%20%28single-precision%29)))

(event EventPostLogin
  (params (NewPlayer :type Player%20Controller%20Object%20Reference))
  (Development|PrintString "OnPostLogin")
  (bind _asbp_player_controller (Utilities|Casting|CastToBP_PlayerController NewPlayer))
  (Utilities|Array|AddUnique (Variables|Default|GetPlayer%20Controllers) _asbp_player_controller))

(fn ConstructionScript)