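; Player controller for Ball of the Wild that sets up the player's pawn and UI on MultiplayerMap1.
; On BeginPlay in that level, it spawns the Character class stored in the game instance at the origin and possesses it.
; It then adds score, timer and multiplayer select widgets, plus a stamina bar outside Challenge mode, and hides the cursor.
; An unconnected branch that destroys the last BP_ThirdPersonCharacter never runs.
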(event EventBeginPlay
  (bind _returnvalue (Game|GetCurrentLevelName true))
  (if (not (Utilities|Enum|NotEqual(Enum) _returnvalue "MultiplayerMap1"))
    (bind _asbp_ball_of_the_wild_game_instance (Utilities|Casting|CastToBP_BallOfTheWildGameInstance (Game|GetGameInstance)))
    (bind _returnvalue_2 (Game|SpawnActorfromClass (Variables|/Game/BP_BallOfTheWildGameInstance.BP_BallOfTheWildGameInstance_C|GetCharacter _asbp_ball_of_the_wild_game_instance) (Math|Transform|MakeTransform "0, 0, 0") "AdjustIfPossibleButAlwaysSpawn" self 0))
    (Pawn|Possess _returnvalue_2)
    (bind _asbp_ball_of_the_wild_game_instance_2 (Utilities|Casting|CastToBP_BallOfTheWildGameInstance (Game|GetGameInstance)))
    (if (Utilities|Enum|Equal(Enum) (Variables|/Game/BP_BallOfTheWildGameInstance.BP_BallOfTheWildGameInstance_C|GetGame%20Mode _asbp_ball_of_the_wild_game_instance_2) "Challenge")
      _
      (else
        (bind _returnvalue_3 (UserInterface|CreateWidget "/Game/Stamina_Bar.Stamina_Bar_C"))
        (UserInterface|Viewport|AddtoViewport _returnvalue_3 0)))
    (bind _returnvalue_4 (UserInterface|CreateWidget "/Game/TeamScore.TeamScore_C"))
    (UserInterface|Viewport|AddtoViewport _returnvalue_4 0)
    (bind _returnvalue_5 (UserInterface|CreateWidget "/Game/Timer_UI.Timer_UI_C"))
    (UserInterface|Viewport|AddtoViewport _returnvalue_5 0)
    (bind _returnvalue_6 (UserInterface|CreateWidget "/Game/MultiplayerSelectWidget.MultiplayerSelectWidget_C"))
    (UserInterface|Viewport|AddtoViewport _returnvalue_6 0)
    (Variables|/Script/Engine.PlayerController|SetbShowMouseCursor self false)))

(event EventTick
  (params (DeltaSeconds :type Float%20%28single-precision%29)))

(fn ConstructionScript)